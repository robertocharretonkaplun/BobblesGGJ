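; BP_Pato is a duck Blueprint in the DrivableBoat folder, holding steering and health helper functions for a water vehicle.
; UpdateMotorAngle smoothly interpolates the steering wheel toward the right-axis input scaled by max steer angle, or toward center when off water, using frame delta time.
; ManageHealth only gates zero health through a DoOnce with no following action, ignoring Damage.
; EventGraph holds only disconnected rotation, velocity and player-index fragments.
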(fn `ManageHealth`
  (params (Damage :type "Float (double-precision)"))
  (locals (L_CurrentHealth :type "Float (double-precision)"))
  (bind _output_get (set `local.L_CurrentHealth` (`self.DuckHealth`)))
  (if (<= _output_get 0.0)
    (`/Engine/EditorBlueprintResources/StandardMacros.DoOnce` false)))

(fn `UpdateMotorAngle`
  ;[1 1 1] Change steering wheel angle
  (set `self.CurrentSteeringWheel` (`KismetMathLibrary.Lerp` (`self.CurrentSteeringWheel`) (* (select `bool` (`self.OnWater`) :`true` (`self.MoveRightAxis`)) (`self.Max Steer Angle`)) (`KismetMathLibrary.FClamp` (* (`GameplayStatics.GetWorldDeltaSeconds`) (`self.SteeringChangingSpeed`))))))

(fn `UserConstructionScript`)