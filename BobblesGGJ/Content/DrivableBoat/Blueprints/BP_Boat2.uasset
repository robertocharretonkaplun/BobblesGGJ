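; Drivable boat pawn, possessed on BeginPlay and steered with arrow keys, with duck health and respawn.
; Tick integrates throttle, damping and anti-slide into a custom horizontal velocity applied by actor offset, adding steering yaw, interpolated pitch/roll and gravity force.
; Hits push physics objects or bounce the boat, and Left Shift adds an impulse.
; ManageHealth ignores damage amount; zero health triggers camera fade and respawn, while camera-look and Left-release logic are unwired.
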(event `Apply Gravity`
  ;[1 1 1] Gravity
  (`PrimitiveComponent.AddForce` (`self.RootMesh`) (* (0.0 0.0 -1.0) (`self.Gravity`)) "None" true))

(event `self.ReceiveHit`
  (params (MyComp :type "PrimitiveComponent Object Reference") (Other :type "Actor Object Reference") (OtherComp :type "PrimitiveComponent Object Reference") (bSelfMoved :type Boolean) (HitLocation :type "Vector Structure") (HitNormal :type "Vector Structure") (NormalImpulse :type "Vector Structure") (Hit :type "HitResult Structure (by ref)"))
  (bind _current_horizontal_velocity (`self.Current Horizontal Velocity`))
  ;[1 1 1] Change velocity if boat impact
  (if (`SceneComponent.IsSimulatingPhysics` OtherComp "None")
    (`PrimitiveComponent.AddForce` OtherComp (* _current_horizontal_velocity (`PrimitiveComponent.GetMass` (`self.RootMesh`))) "None" false)
    (set `self.Current Horizontal Velocity` (* _current_horizontal_velocity 0.9))
    (else
      (set `self.Current Horizontal Velocity` (* HitNormal (* (`KismetMathLibrary.VSize` _current_horizontal_velocity) 0.3))))))

(event `self.ReceiveBeginPlay`
  ;[1 1 1] Possess on BeginPlay
  (`Controller.Possess` (`GameplayStatics.GetPlayerController` 0) self))

(event `Key|Up`
  (params (Key :type "Key Structure"))
  (:`Pressed`
    ;[1 1 1] Input
    (set `self.MoveForwardAxis` 1.0)
    (goto _label_3 :!via `Close`))
  (:`Released`
    (`|ExecutionSequence`
      (:`then_0`
        (`/Engine/EditorBlueprintResources/StandardMacros.Gate` false :!label _label
          (:`Exit`
            (set `self.MoveForwardAxis` 0.0 :!label _label_2))))
      (:`then_1`
        (goto _label_3 :!via `Open`)))))

(event `Key|Down`
  (params (Key :type "Key Structure"))
  (:`Pressed`
    ;[1 1 1] Input
    (set `self.MoveForwardAxis` -1.0)
    (goto _label :!via `Close`))
  (:`Released`
    (`|ExecutionSequence`
      (:`then_0`
        (`/Engine/EditorBlueprintResources/StandardMacros.Gate` false :!label _label_3
          (:`Exit`
            (goto _label_2))))
      (:`then_1`
        (goto _label :!via `Open`)))))

(event `Key|Right`
  (params (Key :type "Key Structure"))
  (:`Pressed`
    ;[1 1 1] Input
    (set `self.MoveRightAxis` 1.0)
    (`/Engine/EditorBlueprintResources/StandardMacros.Gate` false :!via `Close` :!label _label_4
      (:`Exit`
        (set `self.MoveRightAxis` 0.0 :!label _label_5))))
  (:`Released`
    (`|ExecutionSequence`
      (:`then_0`
        (`/Engine/EditorBlueprintResources/StandardMacros.Gate` false :!label _label_6
          (:`Exit`
            (goto _label_5))))
      (:`then_1`
        (goto _label_4 :!via `Open`)))))

(event `Key|Left`
  (params (Key :type "Key Structure"))
  (:`Pressed`
    ;[1 1 1] Input
    (set `self.MoveRightAxis` -1.0)
    (goto _label_6 :!via `Close`)))

(event `self.ReceiveTick`
  (params (DeltaSeconds :type "Float (single-precision)"))
  (bind _currentforce (`self.CurrentForce`))
  (bind _pitchwhenmoving (`self.PitchWhenMoving`))
  (bind _maxspeed (`self.MaxSpeed`))
  (bind _currentsteeringwheel (`self.CurrentSteeringWheel`))
  (bind _max_steer_angle (`self.Max Steer Angle`))
  (bind _current_horizontal_velocity (`self.Current Horizontal Velocity`))
  (bind _rootmesh (`self.RootMesh`))
  (bind _returnvalue (/ (`self.Acceleration`) 1.5))
  (bind (_relativerotation_roll _relativerotation_pitch _relativerotation_yaw) (`KismetMathLibrary.BreakRotator` (`SceneComponent.RelativeRotation` _rootmesh)))
  (bind (_returnvalue_x _returnvalue_y) (`KismetMathLibrary.BreakVector` (`KismetMathLibrary.TransformDirection` (`SceneComponent.K2_GetComponentToWorld` (`self.RootMesh`)) (* (`KismetMathLibrary.MakeVector` (`self.CurrentForce`)) (`GameplayStatics.GetWorldDeltaSeconds`)))))
  (bind (_returnvalue_x_2 _returnvalue_y_2) (`KismetMathLibrary.BreakVector` (+ (+ (+ _current_horizontal_velocity (* _current_horizontal_velocity (* (`self.VelocityDamping`) (`GameplayStatics.GetWorldDeltaSeconds`)))) (* (`self.GetActorRightVector`) (* (* (`self.Current Sliding Speed`) -1.0) (* (`self.Anti Slide`) (`GameplayStatics.GetWorldDeltaSeconds`))))) (`KismetMathLibrary.MakeVector` _returnvalue_x _returnvalue_y))))
  (`|ExecutionSequence`
    (:`then_0`
      ;[1 1 1] Calculate force
      (set `self.CurrentForce` (`KismetMathLibrary.FClamp` (+ (select `bool` (and (< _currentforce _returnvalue) (> _currentforce (* _returnvalue -1.0))) :`false` (select `bool` (> _currentforce 0.0) :`false` (+ _currentforce _returnvalue) :`true` (- _currentforce _returnvalue))) (select `bool` (`self.OnWater`) :`true` (* (`self.MoveForwardAxis`) (`self.Acceleration`)))) (/ _maxspeed (`self.BackwardSpeedMultiplier`)) _maxspeed))
      ;[1 1 1] Move boat
      (bind _output_get (set `self.Current Horizontal Velocity` (`KismetMathLibrary.MakeVector` _returnvalue_x_2 _returnvalue_y_2)))
      (`self.K2_AddActorWorldOffset` (* _output_get (`GameplayStatics.GetWorldDeltaSeconds`)))
      ;[1 1 1] Torque
      (`self.UpdateMotorAngle`)
      (set `self.CurrentPitch` (`KismetMathLibrary.FClamp` (`KismetMathLibrary.Abs` (`KismetMathLibrary.FInterpTo` (`self.CurrentPitch`) (* _pitchwhenmoving (/ (`self.Current Horizontal Speed`) (`self.MaxSpeed`))) (`GameplayStatics.GetWorldDeltaSeconds`) 3.0)) 0.0 _pitchwhenmoving))
      (set `self.CurrentRoll` (`KismetMathLibrary.FClamp` (`KismetMathLibrary.FInterpTo` (`self.CurrentRoll`) (select `bool` (`KismetMathLibrary.NearlyEqual_FloatFloat` _currentsteeringwheel 0.0 0.5) :`false` (* (* (`self.RollWhenSteering`) (/ _currentsteeringwheel (`self.Max Steer Angle`))) (/ (`self.Current Horizontal Speed`) (`self.MaxSpeed`)))) (`GameplayStatics.GetWorldDeltaSeconds`) 3.0) (* -1 _max_steer_angle) _max_steer_angle))
      (`SceneComponent.K2_AddRelativeRotation` _rootmesh (`KismetMathLibrary.MakeRotator` 0.0 0.0 (* (`self.SteeringForce`) (`self.CurrentSteeringWheel`) (`GameplayStatics.GetWorldDeltaSeconds`))) false false)
      (`self.K2_SetActorRelativeRotation` (`KismetMathLibrary.MakeRotator` (`self.CurrentRoll`) (`self.CurrentPitch`) _relativerotation_yaw) false true))
    (:`then_1`)
    (:`then_2`
      ;[1 1 1] Gravity
      (`self.Apply Gravity`))
    (:`then_4`
      ;[1 1 1] Calculate velues
      (set `self.Current Horizontal Speed` (`KismetMathLibrary.VSize` (`KismetMathLibrary.ProjectVectorOnToPlane` (* (- (`self.K2_GetActorLocation`) (`self.LastLocation`)) (/ 1.0 (`GameplayStatics.GetWorldDeltaSeconds`))) (`SceneComponent.GetUpVector` (`self.RootMesh`)))))
      (set `self.Current Sliding Speed` (`KismetMathLibrary.Dot_VectorVector` (`self.Current Horizontal Velocity`) (`self.GetActorRightVector`)))
      (set `self.LastLocation` (`self.K2_GetActorLocation`)))))

(event `Key|LeftShift`
  (params (Key :type "Key Structure"))
  (:`Pressed`
    (if (not (`self.IsDashing`))
      (set `self.IsDashing` true)
      (`PrimitiveComponent.AddVelocityChangeImpulseAtLocation` (`self.RootMesh`) (0.0 50.0 0.0) (0.0 0.0 0.0) "None")))
  (:`Released`
    (`KismetSystemLibrary.Delay` 2.5)
    (set `self.IsDashing` false)))

(event `FadeCamera`
  (params (`Camera Manager` :type "PlayerCameraManager Object Reference") (`Start Fade Time` :type "Float (double-precision)") (`Duration Between` :type "Float (double-precision)") (`End Fade Time` :type "Float (double-precision)"))
  ;[1 0 0] Event Camera Fade
  (`PlayerCameraManager.StartCameraFade` :`self` `Camera Manager` :`ToAlpha` 1.0 :`Duration` `Start Fade Time` :`bHoldWhenFinished` true)
  (`KismetSystemLibrary.Delay` `Duration Between`)
  (`PlayerCameraManager.StartCameraFade` :`self` `Camera Manager` :`FromAlpha` 1.0 :`Duration` `End Fade Time`))

(event `OnDeath`
  (`KismetSystemLibrary.Delay` 0.3)
  (`self.FadeCamera` (`GameplayStatics.GetPlayerCameraManager` 0) 0.5 3.0 0.5)
  (`KismetSystemLibrary.Delay` 2.0)
  (bind _returnvalue (`GameplayStatics.GetActorOfClass` "/Game/Personalized/Blueprints/BP_RespawwnPoint.BP_RespawwnPoint_C"))
  (`self.K2_SetActorTransform` (`/Game/Personalized/Blueprints/BP_RespawwnPoint.RespawnPoint` _returnvalue))
  (`self.SetActorScale3D` (5.0 5.0 5.0))
  (set `self.DuckHealth` 100.0))

(event `self.ReceiveAnyDamage`
  (params (Damage :type "Float (single-precision)") (DamageType :type "DamageType Object Reference") (InstigatedBy :type "Controller Object Reference") (DamageCauser :type "Actor Object Reference"))
  (bind _newhealth (`self.ManageHealth` Damage))
  (set `self.DuckHealth` _newhealth))

(fn `ManageHealth`
  (params (Damage :type "Float (double-precision)"))
  (returns (NewHealth :type "Float (double-precision)"))
  (locals (L_CurrentHealth :type "Float (double-precision)"))
  (bind _output_get (set `local.L_CurrentHealth` (`self.DuckHealth`)))
  (if (<= _output_get 0.0)
    (`/Engine/EditorBlueprintResources/StandardMacros.DoOnce` false
      (:`Completed`
        (`self.OnDeath`)
        (return (`local.L_CurrentHealth`))))))

(fn `UpdateMotorAngle`
  ;[1 1 1] Change steering wheel angle
  (set `self.CurrentSteeringWheel` (`KismetMathLibrary.Lerp` (`self.CurrentSteeringWheel`) (* (select `bool` (`self.OnWater`) :`true` (`self.MoveRightAxis`)) (`self.Max Steer Angle`)) (`KismetMathLibrary.FClamp` (* (`GameplayStatics.GetWorldDeltaSeconds`) (`self.SteeringChangingSpeed`))))))

(fn `UserConstructionScript`)