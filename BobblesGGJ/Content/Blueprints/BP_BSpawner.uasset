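; Spawner actor that periodically spawns a random entry from its BubblesSpawn class list inside a volume.
; BeginPlay starts a looping timer at SpawnInterval, which calls SpawnRandomObject to spawn at a random point within the SpawnArea component's bounds.
; The construction script applies the Scale variable to SpawnArea to size the volume.
; The random index range includes the array length, so it can land one past the last entry.
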(event `self.ReceiveBeginPlay`
  (`KismetSystemLibrary.K2_SetTimer` null "SpawnRandomObject" (`self.SpawnInterval`) true))

(event `SpawnRandomObject`
  (bind _bubblesspawn (`self.BubblesSpawn`))
  (bind (_origin _boxextent) (`KismetSystemLibrary.GetComponentBounds` (`self.SpawnArea`)))
  (`|SpawnActorFromClass` (`|GetArrayItem` _bubblesspawn (`KismetMathLibrary.RandomIntegerInRange` 0 (`KismetArrayLibrary.Array_Length` _bubblesspawn))) (`KismetMathLibrary.Conv_VectorToTransform` (`KismetMathLibrary.RandomPointInBoundingBox` _origin _boxextent)) "Undefined" "MultiplyWithRoot" null null))

(fn `UserConstructionScript`
  (`SceneComponent.SetRelativeScale3D` (`self.SpawnArea`) (`self.Scale`)))