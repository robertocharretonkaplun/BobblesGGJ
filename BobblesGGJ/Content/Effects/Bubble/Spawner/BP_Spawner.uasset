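; BP_Spawner periodically spawns bubble actors (BP_Burbuja) at random TargetPoints in the level.
; Tick feeds a Delay, which ignores calls while counting down, so the Spawnear event fires roughly every five seconds.
; Spawnear loops up to Totalburbujas1, re-querying all TargetPoint actors each iteration and spawning a bubble at a randomly chosen one's transform.
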(event `self.ReceiveTick`
  (params (DeltaSeconds :type "Float (single-precision)"))
  (`KismetSystemLibrary.Delay` 5.0)
  (`self.Spawnear`))

(event `Spawnear`
  (for _ (range (+ (`self.Totalburbujas-1`) 1))
    (bind _outactors (`GameplayStatics.GetAllActorsOfClass` "/Script/Engine.TargetPoint"))
    (`|SpawnActorFromClass` "/Game/Effects/Bubble/BP_Burbuja.BP_Burbuja_C" (`self.GetTransform` (`|GetArrayItem` _outactors (`KismetMathLibrary.RandomIntegerInRange` 0 (`KismetArrayLibrary.Array_LastIndex` _outactors)))) "Undefined" "MultiplyWithRoot" null null)))

(fn `UserConstructionScript`)