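; BP_Burbuja is a bubble actor that grows and rises until it pops, firing a radial force impulse and destroying itself.
; It pops when BP_ThirdPersonCharacter overlaps its mesh or when its elapsed-time counter reaches TiempoDeVida.
; Tick drives both the counter and the scale and height animation through Delay nodes, so they advance in steps rather than every frame.
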(event `contadorVida`
  ;[1 1 1] Tiempo de vida
  (`KismetSystemLibrary.Delay` 0.2)
  (set `self.tiempoTrancurrido` (+ (`self.tiempoTrancurrido`) 0.1)))

(event `ExplotarBurbuja`
  (bind _radialforce (`self.RadialForce`))
  (`ActorComponent.Activate` _radialforce false)
  (`RadialForceComponent.FireImpulse` _radialforce)
  (`self.K2_DestroyActor`))

(event `self.mesh.OnComponentBeginOverlap`
  (params (OverlappedComponent :type "PrimitiveComponent Object Reference") (OtherActor :type "Actor Object Reference") (OtherComp :type "PrimitiveComponent Object Reference") (OtherBodyIndex :type Integer) (bFromSweep :type Boolean) (SweepResult :type "HitResult Structure (by ref)"))
  (cast `/Game/ThirdPerson/Blueprints/BP_ThirdPersonCharacter` OtherActor)
  (`self.ExplotarBurbuja`))

(event `self.ReceiveTick`
  (params (DeltaSeconds :type "Float (single-precision)"))
  ;[1 1 1] Tick
  (`self.contadorVida`)
  (if (>= (`self.tiempoTrancurrido`) (`self.tiempoDeVida`))
    (`self.ExplotarBurbuja`)
    (else
      (`KismetSystemLibrary.Delay` 0.4)
      (`self.AnimBurbuja`))))

(event `AnimBurbuja`
  (bind _mesh (`self.mesh`))
  (bind _returnvalue_location (`KismetMathLibrary.BreakTransform` (`SceneComponent.GetRelativeTransform` (`self.mesh`))))
  ;[1 1 1] Animaciones de burbuja
  ;;[1 1 1] Las hace mas grandes
  (bind _output_get (set `self.esfera escala` (+ (`self.esfera escala`) (* (stale `self.ReceiveTick` DeltaSeconds) 5.0))))
  (`SceneComponent.SetWorldScale3D` _mesh _output_get)
  ;;[1 1 1] Movimiento en Z
  (bind _output_get_2 (set `self.Return Value Location` (+ _returnvalue_location (0.0 0.0 20.0))))
  (`SceneComponent.K2_SetRelativeLocation` _mesh _output_get_2 false false))

(fn `UserConstructionScript`)